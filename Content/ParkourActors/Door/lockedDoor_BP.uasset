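; Locked door actor that the ThirdPersonCharacter can open and close only while holding a key.
; A box overlap stores the character, enables player input on the door and opens a gate, reversing input and gate on exit.
; InteractObjects plays a locked sound without a key; otherwise it passes the gate into a FlipFlop that plays or reverses a timeline lerping door yaw, with open and close sounds.
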(event `/Game/Blueprints/InteractInterface.InteractObjects`
  (params (Player :type "Character Object Reference"))
  (bind _returnvalue (`self.K2_GetActorLocation`))
  (if (`/Game/ThirdPersonBP/Blueprints/ThirdPersonCharacter.hasKey` (stale `self.Box.OnComponentBeginOverlap` _asthird_person_character))
    (`/Engine/EditorBlueprintResources/StandardMacros.Gate` true :!label _label
      (:`Exit`
        (`/Engine/EditorBlueprintResources/StandardMacros.FlipFlop`
          (:`A`
            (`GameplayStatics.PlaySoundAtLocation` "/Game/ParkourActors/Door/doorOpen.doorOpen" _returnvalue (struct) 1.0 1.0 0.0 null null null)
            (bind (_direction _open_closed) (`Timeline|Open/Closed Door` :!label _label_2)
              (:`Update`
                (`SceneComponent.K2_SetRelativeRotation` (`self.door`) (`KismetMathLibrary.MakeRotator` 0.0 0.0 (`KismetMathLibrary.Lerp` (`self.ClosedAngle`) (`self.OpenAngle`) _open_closed)) false false))))
          (:`B`
            (`GameplayStatics.PlaySoundAtLocation` "/Game/ParkourActors/Door/closedDoor.closedDoor" _returnvalue (struct) 1.0 1.0 0.0 null null null)
            (goto _label_2 :!via `Reverse`)))))
    (else
      (`GameplayStatics.PlaySoundAtLocation` "/Game/ParkourActors/Door/lockeddoor.lockedDoor" _returnvalue (struct) 1.0 1.0 0.0 null null null))))

(event `self.Box.OnComponentBeginOverlap`
  (params (OverlappedComponent :type "PrimitiveComponent Object Reference") (OtherActor :type "Actor Object Reference") (OtherComp :type "PrimitiveComponent Object Reference") (OtherBodyIndex :type Integer) (bFromSweep :type Boolean) (SweepResult :type "HitResult Structure (by ref)"))
  (bind _asthird_person_character (cast `/Game/ThirdPersonBP/Blueprints/ThirdPersonCharacter` OtherActor))
  (`self.EnableInput` (`GameplayStatics.GetPlayerController` 0))
  (goto _label :!via `Open`))

(event `self.Box.OnComponentEndOverlap`
  (params (OverlappedComponent :type "PrimitiveComponent Object Reference") (OtherActor :type "Actor Object Reference") (OtherComp :type "PrimitiveComponent Object Reference") (OtherBodyIndex :type Integer))
  (cast `/Game/ThirdPersonBP/Blueprints/ThirdPersonCharacter` OtherActor)
  (`self.DisableInput` (`GameplayStatics.GetPlayerController` 0))
  (goto _label :!via `Close`))

(fn `UserConstructionScript`)