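; Base weapon actor for guns the third-person player picks up, fires and reloads, with an overlap-driven interaction prompt.
; Gated firing line-traces from the weapon's arrow toward camera aim, plays effects and recoil, spends ammo and sends damage through the TakeDamage interface.
; Manual or automatic reloads wait out a montage, then draw from the player's WeaponSystemComponent ammo pool.
; SetWeaponState switches collision per state, moving dropped weapons to a downward trace's hit.
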(event `StartFire`
  (bind (_start _end) (`self.StartAndEndPoint`))
  (bind (_weaponstruct_weaponname _weaponstruct_weaponenum _weaponstruct_weaponclass _weaponstruct_magsize _weaponstruct_currentammo) (break `/Game/Blueprints/Weapons/WeaponStruct` (`self.WeaponStruct`)))
  (`self.AutoReload`)
  (`|ExecutionSequence`
    (:`then_0`
      (goto _label :!via `Open`))
    (:`then_1`
      (`/Engine/EditorBlueprintResources/StandardMacros.Gate` true :!label _label
        (:`Exit`
          (if (> _weaponstruct_currentammo 0)
            (bind (_outhit _returnvalue) (`KismetSystemLibrary.LineTraceSingle` _start _end "TraceTypeQuery3" false (`|MakeArray` (`self.Interactor`))))
            (bind (_bblockinghit _binitialoverlap _time _distance _location _impactpoint _normal _impactnormal _physmat _hitactor _hitcomponent _hitbonename _hititem _elementindex _faceindex _tracestart _traceend) (`GameplayStatics.BreakHitResult` _outhit))
            (`self.GunEffects` _returnvalue _impactpoint (select `bool` _returnvalue :`false` _traceend :`true` _impactpoint))
            (`self.RemoveAmmoFromGun`)
            (`self.AddDamageToHitObject` _hitactor _outhit)))))))

(event `StopFire`
  (`self.AutoReload`)
  (goto _label :!via `Close`))

(event `Simulation`
  (bind _returnvalue (`self.K2_GetActorLocation`))
  (bind _outhit (`KismetSystemLibrary.LineTraceSingle` _returnvalue (`KismetMathLibrary.MakeVector` (.x _returnvalue) (.y _returnvalue) (* (.z _returnvalue) -50.0)) "TraceTypeQuery1"))
  (`KismetSystemLibrary.MoveComponentTo` (`self.DefaultSceneRoot`) (+ (`.Location` (`GameplayStatics.BreakHitResult` _outhit)) (0.0 0.0 4.0)) (struct :`Pitch` 90.0 :`Roll` 90.0)))

(event `/Game/Blueprints/InteractInterface.Interact`
  (params (Interactor :type "Actor Object Reference"))
  (bind _output_get (set `self.Interactor` Interactor))
  (`/Game/Blueprints/Weapons/Weapon_System_Component.PickUpWeapon` (`self.GetComponentByClass` Interactor "/Game/Blueprints/Weapons/Weapon_System_Component.Weapon_System_Component_C") self)
  (bind _asthird_person_character (cast `/Game/ThirdPersonBP/Blueprints/ThirdPersonCharacter` _output_get))
  (set `self.PlayerRef` _asthird_person_character))

(event `self.InteractionArea.OnComponentBeginOverlap`
  (params (OverlappedComponent :type "PrimitiveComponent Object Reference") (OtherActor :type "Actor Object Reference") (OtherComp :type "PrimitiveComponent Object Reference") (OtherBodyIndex :type Integer) (bFromSweep :type Boolean) (SweepResult :type "HitResult Structure (by ref)"))
  (bind _widget (`self.Widget`))
  (cast `/Game/ThirdPersonBP/Blueprints/ThirdPersonCharacter` OtherActor)
  (set `self.CanPick` true)
  (`self.InteractUI`
    (:`then`
      _)
    (:`else`
      (bind _returnvalue (`|CreateWidget` "/Game/Blueprints/Weapons/UI/InteractWidget.InteractWidget_C" null (`.WeaponName_16_B8FD7EC645FFCAED4E59779F80684BE4` (break `/Game/Blueprints/Weapons/WeaponStruct` (`self.WeaponStruct`)))))
      (set `self.InteractUI` _returnvalue)
      (`WidgetComponent.SetWidget` _widget _returnvalue)))
  (`SceneComponent.SetVisibility` _widget true false))

(event `self.InteractionArea.OnComponentEndOverlap`
  (params (OverlappedComponent :type "PrimitiveComponent Object Reference") (OtherActor :type "Actor Object Reference") (OtherComp :type "PrimitiveComponent Object Reference") (OtherBodyIndex :type Integer))
  (`SceneComponent.SetVisibility` (`self.Widget`) false false)
  (set `self.CanPick` false))

(event `ReloadEvent`
  (`GameplayStatics.PlaySound2D` (`self.ReloadSound`) 1.0 1.0 0.0 null null)
  (bind _returnvalue (`Character.PlayAnimMontage` (`self.PlayerRef`) (`self.reloadMontage`) 1.0 "None"))
  (`KismetSystemLibrary.Delay` _returnvalue)
  (`self.SetBulletsAndReload`)
  (set `self.IsReloading` false))

(event `ReloadButtonEvent`
  (bind ((`MagSize_19_9953F52E4DCC1692F54102B42CB12371` _magsize) (`CurrentAmmo_20_A605F2184A1BC9C05D75AD8AE1A77820` _currentammo)) (break `/Game/Blueprints/Weapons/WeaponStruct` (`self.WeaponStruct`)))
  (if (!= (`.CurrentAmmo_20_A605F2184A1BC9C05D75AD8AE1A77820` (break `/Game/Blueprints/Weapons/WeaponStruct` (`self.WeaponStruct`))) 0)
    (if (!= _magsize _currentammo)
      (if (not (`self.IsReloading`))
        (set `self.IsReloading` true)
        (`self.ReloadEvent`)))))

(event `AutoReload`
  (bind ((`CurrentAmmo_20_A605F2184A1BC9C05D75AD8AE1A77820` _currentammo) (`AmmoType_30_E32FA0AE4C4E75A5BF8A7A8DC601CBAC` _ammotype)) (break `/Game/Blueprints/Weapons/WeaponStruct` (`self.WeaponStruct`)))
  (if (and (== _currentammo 0) (> (`BlueprintMapLibrary.Map_Find` (`/Game/Blueprints/Weapons/Weapon_System_Component.AmmoType/TotalAmmo` (`/Game/ThirdPersonBP/Blueprints/ThirdPersonCharacter.Weapon_System_Component` (`self.PlayerRef`))) _ammotype) 0))
    (if (not (`self.IsReloading`))
      (set `self.IsReloading` true)
      (`self.ReloadEvent`))))

(fn `AddDamageToHitObject`
  (params (HitObject :type "Actor Object Reference") (HitEvents :type "HitResult Structure"))
  (if (`KismetSystemLibrary.DoesImplementInterface` HitObject "/Game/Blueprints/TakeDamage.TakeDamage_C")
    (message `/Game/Blueprints/TakeDamage.DoDamage` HitObject (`.Damage_22_563B9BF741C1C57B47AF17827EFB0367` (break `/Game/Blueprints/Weapons/WeaponStruct` (`self.WeaponStruct`))) HitEvents)
    (return)))

(fn `GunEffects`
  (params (DoesHit :type Boolean) (ImpactPoint :type "Vector Structure") (TraceEnd :type "Vector Structure"))
  (bind _weaponmesh (`/Game/Blueprints/Weapons/MasterWeapon.WeaponMesh` (`/Game/Blueprints/Weapons/Weapon_System_Component.InHandWeapon` (`/Game/ThirdPersonBP/Blueprints/ThirdPersonCharacter.Weapon_System_Component` (`self.PlayerRef`)))))
  (bind _returnvalue (`SceneComponent.GetSocketLocation` _weaponmesh "Muzzle"))
  (`GameplayStatics.PlaySound2D` (`self.ShootSound`) 1.0 1.0 0.0 null null)
  (`Character.PlayAnimMontage` (`self.PlayerRef`) (`self.FireAnimation`) 1.0 "None")
  (`GameplayStatics.SpawnEmitterAttached` "/Game/Blueprints/Weapons/Effects/MuzzleFlash.MuzzleFlash" _weaponmesh "Muzzle" (0.0 0.0 0.0) (struct) (1.0 1.0 1.0) "SnapToTargetIncludingScale")
  (`|SpawnActorFromClass` "/Game/Blueprints/Weapons/Effects/SelfProjectile/ProjectileTrace.ProjectileTrace_C" (`KismetMathLibrary.MakeTransform` _returnvalue (`KismetMathLibrary.FindLookAtRotation` _returnvalue (`local.TraceEnd`))) "Undefined" "OverrideRootScale" null null)
  (`Pawn.AddControllerPitchInput` (`self.PlayerRef`) (* (`self.Recoil`) -1.0))
  (return))

(fn `RemoveAmmoFromGun`
  (bind _weaponstruct (`self.WeaponStruct`))
  (setmembers `/Game/Blueprints/Weapons/WeaponStruct` :`StructRef` _weaponstruct :`CurrentAmmo` (- (`.CurrentAmmo_20_A605F2184A1BC9C05D75AD8AE1A77820` (break `/Game/Blueprints/Weapons/WeaponStruct` _weaponstruct)) 1))
  (return))

(fn `SetBulletsAndReload`
  (bind _neededtoammo (`self.neededToAmmo`))
  (bind _weaponstruct (`self.WeaponStruct`))
  (bind (_weaponname _weaponenum _weaponclass _magsize _currentammo _damage _weaponimage _ismeleeweapon _ammotype) (break `/Game/Blueprints/Weapons/WeaponStruct` (`self.WeaponStruct`)))
  (bind ((`MagSize_19_9953F52E4DCC1692F54102B42CB12371` _magsize_2) (`AmmoType_30_E32FA0AE4C4E75A5BF8A7A8DC601CBAC` _ammotype_2)) (break `/Game/Blueprints/Weapons/WeaponStruct` _weaponstruct))
  (bind ((`CurrentAmmo_20_A605F2184A1BC9C05D75AD8AE1A77820` _currentammo_2) (`AmmoType_30_E32FA0AE4C4E75A5BF8A7A8DC601CBAC` _ammotype_3)) (break `/Game/Blueprints/Weapons/WeaponStruct` _weaponstruct))
  (bind _ammotype_totalammo (`/Game/Blueprints/Weapons/Weapon_System_Component.AmmoType/TotalAmmo` (`/Game/ThirdPersonBP/Blueprints/ThirdPersonCharacter.Weapon_System_Component` (`self.PlayerRef`))))
  (bind _value (`BlueprintMapLibrary.Map_Find` (`/Game/Blueprints/Weapons/Weapon_System_Component.AmmoType/TotalAmmo` (`/Game/ThirdPersonBP/Blueprints/ThirdPersonCharacter.Weapon_System_Component` (`self.PlayerRef`))) (`.AmmoType_30_E32FA0AE4C4E75A5BF8A7A8DC601CBAC` (break `/Game/Blueprints/Weapons/WeaponStruct` (`self.WeaponStruct`)))))
  (if (> (`BlueprintMapLibrary.Map_Find` (`/Game/Blueprints/Weapons/Weapon_System_Component.AmmoType/TotalAmmo` (`/Game/ThirdPersonBP/Blueprints/ThirdPersonCharacter.Weapon_System_Component` (`self.PlayerRef`))) _ammotype) 0)
    (set `self.neededToAmmo` (- _magsize _currentammo))
    (if (<= _value _neededtoammo)
      (setmembers `/Game/Blueprints/Weapons/WeaponStruct` :`StructRef` _weaponstruct :`CurrentAmmo` (+ _currentammo_2 (`BlueprintMapLibrary.Map_Find` _ammotype_totalammo _ammotype_3)))
      (`BlueprintMapLibrary.Map_Add` _ammotype_totalammo _ammotype_3)
      (else
        (setmembers `/Game/Blueprints/Weapons/WeaponStruct` :`StructRef` _weaponstruct :`CurrentAmmo` _magsize_2)
        (`BlueprintMapLibrary.Map_Add` (`/Game/Blueprints/Weapons/Weapon_System_Component.AmmoType/TotalAmmo` (`/Game/ThirdPersonBP/Blueprints/ThirdPersonCharacter.Weapon_System_Component` (`self.PlayerRef`))) _ammotype_2 (- _value _neededtoammo))))))

(fn `SetWeaponState`
  (params (WeaponState :type "/Game/Blueprints/Weapons/E_WeaponState Enum" :default "NewEnumerator0"))
  (bind _weaponmesh (`self.WeaponMesh`))
  (bind _weaponmesh_2 (`self.WeaponMesh`))
  (bind _returnvalue_location (`KismetMathLibrary.BreakTransform` (`SceneComponent.GetSocketTransform` _weaponmesh_2 "Handle" "RTS_Component")))
  (switch `/Game/Blueprints/Weapons/E_WeaponState` WeaponState
    (:`NewEnumerator0`
      (`PrimitiveComponent.SetCollisionProfileName` (`self.InteractionArea`) "OverlapAllDynamic" true)
      (`PrimitiveComponent.SetCollisionProfileName` (`self.WeaponMesh`) "DroppedGun" true)
      (`self.Simulation`))
    (:`NewEnumerator1`
      (`PrimitiveComponent.SetCollisionProfileName` (`self.InteractionArea`) "NoCollision" true)
      (`PrimitiveComponent.SetCollisionProfileName` (`self.WeaponMesh`) "NoCollision" true)
      (`PrimitiveComponent.SetSimulatePhysics` _weaponmesh false)
      (`SceneComponent.ResetRelativeTransform` _weaponmesh)
      (`SceneComponent.K2_SetRelativeLocation` _weaponmesh_2 (* _returnvalue_location -1.0) false false))
    (:`NewEnumerator2`
      (`PrimitiveComponent.SetCollisionProfileName` (`self.InteractionArea`) "NoCollision" true)
      (`PrimitiveComponent.SetCollisionProfileName` (`self.WeaponMesh`) "NoCollision" true)
      (`PrimitiveComponent.SetSimulatePhysics` (`self.WeaponMesh`) false))))

(fn `StartAndEndPoint`
  (returns (Start :type "Vector Structure") (End :type "Vector Structure"))
  (bind _arrow (`self.Arrow`))
  (bind _followcamera (`/Game/ThirdPersonBP/Blueprints/ThirdPersonCharacter.FollowCamera` (`self.PlayerRef`)))
  (return (+ (`SceneComponent.K2_GetComponentLocation` _arrow) (`KismetMathLibrary.GetForwardVector` (`SceneComponent.K2_GetComponentRotation` _arrow))) (+ (`SceneComponent.K2_GetComponentLocation` _followcamera) (* (`KismetMathLibrary.GetForwardVector` (`SceneComponent.K2_GetComponentRotation` _followcamera)) (`self.Range`)))))

(fn `UserConstructionScript`
  (bind (_weaponstruct_weaponname _weaponstruct_weaponenum _weaponstruct_weaponclass _weaponstruct_magsize _weaponstruct_currentammo _weaponstruct_damage _weaponstruct_weaponimage _weaponstruct_ismeleeweapon _weaponstruct_ammotype) (break `/Game/Blueprints/Weapons/WeaponStruct` (`self.WeaponStruct`)))
  (setmembers `/Game/Blueprints/Weapons/WeaponStruct` :`StructRef` (`self.WeaponStruct`) :`WeaponName` _weaponstruct_weaponname :`WeaponEnum` _weaponstruct_weaponenum :`WeaponClass` (`GameplayStatics.GetObjectClass` self) :`MagSize` _weaponstruct_magsize :`CurrentAmmo` _weaponstruct_currentammo :`Damage` _weaponstruct_damage :`WeaponImage` _weaponstruct_weaponimage :`IsMeleeWeapon` _weaponstruct_ismeleeweapon :`AmmoType` _weaponstruct_ammotype))