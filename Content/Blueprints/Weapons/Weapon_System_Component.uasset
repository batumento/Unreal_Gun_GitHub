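; Weapon inventory component for player 0's ThirdPersonCharacter, handling pickup, drop, equip, swap and sheathe across two rifle, one pistol and one melee holster.
; PickUpWeapon routes by weapon type to holster checks, which drop or stow weapons and retry recursively when full.
; Pickups auto-equip through EquipEvent, which acts on WeaponInput, also set by WeaponTypeAnim after validating slot requests.
; Equip changes snap weapons between mesh sockets and update weapon state and equipped flags.
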(event `self.ReceiveBeginPlay`
  (bind _asthird_person_character (cast `/Game/ThirdPersonBP/Blueprints/ThirdPersonCharacter` (`GameplayStatics.GetPlayerCharacter` 0)))
  (set `self.PlayerRef` _asthird_person_character))

(event `EquipEvent`
  (bind _weaponinput (`self.WeaponInput`))
  (bind _weaponinput_2 (`self.WeaponInput`))
  (bind _weapon (`self.InputBasedOnWeapon` _weaponinput_2))
  (if (`|EnumInequality` (`self.WeaponInput`) "NewEnumerator0")
    (if (`self.HasWeaponEquipped`)
      (if (`|EnumInequality` _weaponinput_2 "NewEnumerator5")
        (`self.SwapWeapon` _weapon)
        (else
          (`self.Equip/Unequip` _weapon)
          (set `self.RifleEquipped` false)
          (set `self.PistolEquipped` false)
          (set `self.MeleeWeaponEquipped` false)))
      (elif (`|EnumInequality` _weaponinput "NewEnumerator5")
        (`self.Equip/Unequip` (`self.InputBasedOnWeapon` _weaponinput) true)))))

(fn `AttachWeaponToPlayer`
  (params (TheWeapon :type "/Game/Blueprints/Weapons/MasterWeapon Object Reference") (Holster :type Name))
  (`Actor.K2_AttachToComponent` TheWeapon (`Character.Mesh` (`self.PlayerRef`)) Holster "SnapToTarget" "SnapToTarget" "SnapToTarget" true)
  (`/Game/Blueprints/Weapons/MasterWeapon.SetWeaponState` TheWeapon "NewEnumerator1")
  (bind _weaponslot (`self.GetSlotBasedOnWeapon` (`local.TheWeapon`)))
  (set `self.WeaponInput` _weaponslot)
  (`self.EquipEvent`))

(fn `DropWeapon`
  (params (WeaponToDrop :type "/Game/Blueprints/Weapons/MasterWeapon Object Reference"))
  (locals (WeaponSlot :type "/Game/Blueprints/Weapons/E_WeaponInput Enum" :default "NewEnumerator0"))
  (bind _weapontodrop (`local.WeaponToDrop`))
  (bind _weaponslot (`self.GetSlotBasedOnWeapon` WeaponToDrop))
  (set `local.WeaponSlot` _weaponslot)
  (`Actor.K2_DetachFromActor` _weapontodrop "KeepWorld" "KeepWorld" "KeepWorld")
  (`/Game/Blueprints/Weapons/MasterWeapon.SetWeaponState` _weapontodrop "NewEnumerator0")
  (set `self.InHandWeapon` null)
  (switch `/Game/Blueprints/Weapons/E_WeaponInput` (`local.WeaponSlot`)
    (:`NewEnumerator1`
      (set `self.PrimaryHolster` null)
      (set `self.RifleEquipped` false))
    (:`NewEnumerator2`
      (set `self.SecondaryHolster` null)
      (set `self.RifleEquipped` false))
    (:`NewEnumerator3`
      (set `self.PistolHolster` null)
      (set `self.PistolEquipped` false))
    (:`NewEnumerator4`
      (set `self.MeleeHolster` null)
      (set `self.MeleeWeaponEquipped` false)))
  (return))

(fn `Equip/Unequip`
  (params (TheWeapon :type "/Game/Blueprints/Weapons/MasterWeapon Object Reference") (WantToEquip :type Boolean))
  (locals (TheWeaponSlot :type "/Game/Blueprints/Weapons/E_WeaponInput Enum" :default "NewEnumerator0"))
  (bind _theweapon (`local.TheWeapon`))
  (bind _weaponslot (`self.GetSlotBasedOnWeapon` TheWeapon))
  (set `local.TheWeaponSlot` _weaponslot)
  (`Actor.K2_AttachToComponent` (`local.TheWeapon`) (`Character.Mesh` (`self.PlayerRef`)) (select `bool` (`local.WantToEquip`) :`false` (select `/Game/Blueprints/Weapons/E_WeaponInput` (`local.TheWeaponSlot`) :`NewEnumerator1` "Holster1" :`NewEnumerator2` "Holster2" :`NewEnumerator3` "PistolHolster" :`NewEnumerator4` "MeleeHolster" :!type "Name") :`true` "InHand") "SnapToTarget" "SnapToTarget" "SnapToTarget" true)
  (switch `/Game/Blueprints/Weapons/E_WeaponInput` (`local.TheWeaponSlot`)
    (:`NewEnumerator1`
      (set `self.RifleEquipped` true))
    (:`NewEnumerator2`
      (set `self.RifleEquipped` true))
    (:`NewEnumerator3`
      (set `self.PistolEquipped` true))
    (:`NewEnumerator4`
      (set `self.MeleeWeaponEquipped` true)))
  (if (`local.WantToEquip`)
    (set `self.InHandWeapon` _theweapon)
    (`/Game/Blueprints/Weapons/MasterWeapon.SetWeaponState` _theweapon "NewEnumerator2")
    (return)
    (else
      (`/Game/Blueprints/Weapons/MasterWeapon.SetWeaponState` (`local.TheWeapon`) "NewEnumerator1")
      (set `self.InHandWeapon` null)
      (set `self.RifleEquipped` false)
      (set `self.PistolEquipped` false)
      (set `self.MeleeWeaponEquipped` false)
      (return))))

(fn `GetSlotBasedOnWeapon`
  (params (TheWeapon :type "/Game/Blueprints/Weapons/MasterWeapon Object Reference"))
  (returns (WeaponSlot :type "/Game/Blueprints/Weapons/E_WeaponInput Enum") (HolsterName :type Name))
  (if (and (`KismetSystemLibrary.IsValid` (`self.PrimaryHolster`)) (== (`local.TheWeapon`) (`self.PrimaryHolster`)))
    (return "NewEnumerator1" "Holster1")
    (elif (and (`KismetSystemLibrary.IsValid` (`self.SecondaryHolster`)) (== (`local.TheWeapon`) (`self.SecondaryHolster`)))
      (return "NewEnumerator2" "Holster2")
      (elif (and (`KismetSystemLibrary.IsValid` (`self.PistolHolster`)) (== (`local.TheWeapon`) (`self.PistolHolster`)))
        (return "NewEnumerator3" "PistolHolster")
        (elif (and (`KismetSystemLibrary.IsValid` (`self.MeleeHolster`)) (== (`local.TheWeapon`) (`self.MeleeHolster`)))
          (return "NewEnumerator4" "MeleeHolster"))))))

(fn `HasWeaponEquipped`
  (returns (IsTrue :type Boolean))
  (return (or (`self.RifleEquipped`) (`self.PistolEquipped`) (`self.MeleeWeaponEquipped`))))

(fn `InputBasedOnWeapon`
  (params (WeaponInput :type "/Game/Blueprints/Weapons/E_WeaponInput Enum" :default "NewEnumerator0"))
  (returns (Weapon :type "/Game/Blueprints/Weapons/MasterWeapon Object Reference"))
  (bind _primaryholster (`self.PrimaryHolster`))
  (bind _secondaryholster (`self.SecondaryHolster`))
  (bind _pistolholster (`self.PistolHolster`))
  (bind _meleeholster (`self.MeleeHolster`))
  (bind _inhandweapon (`self.InHandWeapon`))
  (switch `/Game/Blueprints/Weapons/E_WeaponInput` WeaponInput
    (:`NewEnumerator1`
      (`/Engine/EditorBlueprintResources/StandardMacros.IsValid` _primaryholster
        (:`Is Valid`
          (return _primaryholster))))
    (:`NewEnumerator2`
      (`/Engine/EditorBlueprintResources/StandardMacros.IsValid` _secondaryholster
        (:`Is Valid`
          (return _secondaryholster))))
    (:`NewEnumerator3`
      (`/Engine/EditorBlueprintResources/StandardMacros.IsValid` _pistolholster
        (:`Is Valid`
          (return _pistolholster))))
    (:`NewEnumerator4`
      (`/Engine/EditorBlueprintResources/StandardMacros.IsValid` _meleeholster
        (:`Is Valid`
          (return _meleeholster))))
    (:`NewEnumerator5`
      (`/Engine/EditorBlueprintResources/StandardMacros.IsValid` _inhandweapon
        (:`Is Valid`
          (return _inhandweapon))))))

(fn `PickUpWeapon`
  (params (TheWeapon :type "/Game/Blueprints/Weapons/MasterWeapon Object Reference"))
  (locals (InteractingWeapon :type "/Game/Blueprints/Weapons/MasterWeapon Object Reference"))
  (bind _output_get (set `local.InteractingWeapon` TheWeapon))
  (switch `/Game/Blueprints/Weapons/E_WeaponEnum` (`.WeaponEnum_17_8A3BBA434C6B1C07ACD65C995775CD14` (break `/Game/Blueprints/Weapons/WeaponStruct` (`/Game/Blueprints/Weapons/MasterWeapon.WeaponStruct` _output_get)))
    (:`NewEnumerator1`
      (bind _weapon (`self.CheckRifleHolsterAvaibility` (`local.InteractingWeapon`) :!label _label)
        (:`Full Holster`
          (`self.PickUpWeapon` (`local.InteractingWeapon`)))
        (:`Secondary Holster Empty`
          (bind _output_get_2 (set `self.SecondaryHolster` _weapon))
          (`self.AttachWeaponToPlayer` _output_get_2 (`self.EmptyHolster`)))
        (:`Primary Holster Empty`
          (bind _output_get_3 (set `self.PrimaryHolster` _weapon))
          (`self.AttachWeaponToPlayer` _output_get_3 (`self.EmptyHolster`)))))
    (:`NewEnumerator2`
      (goto _label))
    (:`NewEnumerator3`
      (goto _label))
    (:`NewEnumerator6`
      (goto _label))
    (:`NewEnumerator5`
      (bind _weapon_2 (`self.CheckPistolHolsterAvaibility` (`local.InteractingWeapon`))
        (:`FullPistolHolsterEmpty`
          (`self.PickUpWeapon` (`local.InteractingWeapon`)))
        (:`PistolHolsterEmpty`
          (bind _output_get_4 (set `self.PistolHolster` _weapon_2))
          (`self.AttachWeaponToPlayer` _output_get_4 (`self.EmptyHolster`)))))
    (:`NewEnumerator4`
      (bind _weapon_3 (`self.CheckMeleeHolsterAvaibility` (`local.InteractingWeapon`))
        (:`FullMeleeHolsterEmpty`
          (`self.PickUpWeapon` (`local.InteractingWeapon`)))
        (:`MeleeHolsterEmpty`
          (bind _output_get_5 (set `self.MeleeHolster` _weapon_3))
          (`self.AttachWeaponToPlayer` _output_get_5 (`self.EmptyHolster`)))))))

(fn `SwapWeapon`
  (params (TheWeapon :type "/Game/Blueprints/Weapons/MasterWeapon Object Reference"))
  (locals (NextWeaponSlot :type "/Game/Blueprints/Weapons/E_WeaponInput Enum" :default "NewEnumerator0") (NextWeaponHolster :type Name :default "None") (InHandSlot :type "/Game/Blueprints/Weapons/E_WeaponInput Enum" :default "NewEnumerator0") (InHandHolster :type Name :default "None"))
  (bind _inhandweapon (`self.InHandWeapon`))
  (bind (_weaponslot _holstername) (`self.GetSlotBasedOnWeapon` TheWeapon))
  (set `local.NextWeaponSlot` _weaponslot)
  (set `local.NextWeaponHolster` _holstername)
  (bind (_weaponslot_2 _holstername_2) (`self.GetSlotBasedOnWeapon` (`self.InHandWeapon`)))
  (set `local.InHandSlot` _weaponslot_2)
  (bind _output_get (set `local.InHandHolster` _holstername_2))
  (`Actor.K2_AttachToComponent` _inhandweapon (`Character.Mesh` (`self.PlayerRef`)) _output_get "SnapToTarget" "SnapToTarget" "SnapToTarget" true)
  (`/Game/Blueprints/Weapons/MasterWeapon.SetWeaponState` _inhandweapon "NewEnumerator1")
  (set `self.InHandWeapon` null)
  (set `self.RifleEquipped` false)
  (set `self.PistolEquipped` false)
  (set `self.MeleeWeaponEquipped` false)
  (`self.Equip/Unequip` (`local.TheWeapon`) true))

(fn `WeaponTypeAnim`
  (params (E_Weapon :type "/Game/Blueprints/Weapons/E_WeaponInput Enum" :default "NewEnumerator0"))
  (returns (CanAnimate :type Boolean))
  (bind _inhandweapon (`self.InHandWeapon`))
  (bind _e_weapon (`local.E_Weapon`))
  (switch `/Game/Blueprints/Weapons/E_WeaponInput` E_Weapon
    (:`NewEnumerator1`
      (`/Engine/EditorBlueprintResources/StandardMacros.IsValid` (`self.PrimaryHolster`)
        (:`Is Valid`
          _)
        (:`Is Not Valid`
          (set `self.WeaponInput` "NewEnumerator0" :!label _label)
          (return false))))
    (:`NewEnumerator2`
      (`/Engine/EditorBlueprintResources/StandardMacros.IsValid` (`self.SecondaryHolster`)
        (:`Is Valid`
          _)
        (:`Is Not Valid`
          (goto _label))))
    (:`NewEnumerator3`
      (`/Engine/EditorBlueprintResources/StandardMacros.IsValid` (`self.PistolHolster`)
        (:`Is Valid`
          _)
        (:`Is Not Valid`
          (goto _label))))
    (:`NewEnumerator4`
      (`/Engine/EditorBlueprintResources/StandardMacros.IsValid` (`self.MeleeHolster`)
        (:`Is Valid`
          _)
        (:`Is Not Valid`
          (goto _label))))
    (:`NewEnumerator5`
      (`/Engine/EditorBlueprintResources/StandardMacros.IsValid` (`self.InHandWeapon`)
        (:`Is Valid`
          (set `self.WeaponInput` "NewEnumerator5")
          (return true)))))
  (`/Engine/EditorBlueprintResources/StandardMacros.IsValid` _inhandweapon
    (:`Is Valid`
      (bind _weaponslot (`self.GetSlotBasedOnWeapon` _inhandweapon))
      (if (`|EnumEquality` _weaponslot _e_weapon)
        (set `self.WeaponInput` "NewEnumerator0")
        (return false)
        (else
          _)))
    (:`Is Not Valid`
      _))
  (set `self.WeaponInput` _e_weapon)
  (return true))