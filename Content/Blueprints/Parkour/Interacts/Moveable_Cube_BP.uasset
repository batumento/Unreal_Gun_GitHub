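; A pushable cube for parkour interaction that the third-person character can move by walking into it.
; Two axis trigger volumes enable physics on the cube, switch the character's equipped weapon and set its pushing flag on overlap; leaving turns physics and the flag off.
; It also answers interaction by adding a MovableCube item to the interactor's inventory, and look-at by returning a Turkish "movable box" prompt.
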(event `self.Y Axis Collision.OnComponentBeginOverlap`
  (params (OverlappedComponent :type "PrimitiveComponent Object Reference") (OtherActor :type "Actor Object Reference") (OtherComp :type "PrimitiveComponent Object Reference") (OtherBodyIndex :type Integer) (bFromSweep :type Boolean) (SweepResult :type "HitResult Structure (by ref)"))
  (bind _asthird_person_character (cast `/Game/ThirdPersonBP/Blueprints/ThirdPersonCharacter` OtherActor))
  (`/Game/ThirdPersonBP/Blueprints/ThirdPersonCharacter.EquipWeapon` _asthird_person_character "NewEnumerator5")
  (`PrimitiveComponent.SetSimulatePhysics` (`self.Cube`) true)
  (set `/Game/ThirdPersonBP/Blueprints/ThirdPersonCharacter.isPushing` true _asthird_person_character))

(event `self.Y Axis Collision.OnComponentEndOverlap`
  (params (OverlappedComponent :type "PrimitiveComponent Object Reference") (OtherActor :type "Actor Object Reference") (OtherComp :type "PrimitiveComponent Object Reference") (OtherBodyIndex :type Integer))
  (bind _asthird_person_character (cast `/Game/ThirdPersonBP/Blueprints/ThirdPersonCharacter` OtherActor))
  (`PrimitiveComponent.SetSimulatePhysics` (`self.Cube`) false)
  (set `/Game/ThirdPersonBP/Blueprints/ThirdPersonCharacter.isPushing` false _asthird_person_character))

(event `self.X Axis Collision1.OnComponentBeginOverlap`
  (params (OverlappedComponent :type "PrimitiveComponent Object Reference") (OtherActor :type "Actor Object Reference") (OtherComp :type "PrimitiveComponent Object Reference") (OtherBodyIndex :type Integer) (bFromSweep :type Boolean) (SweepResult :type "HitResult Structure (by ref)"))
  (bind _asthird_person_character (cast `/Game/ThirdPersonBP/Blueprints/ThirdPersonCharacter` OtherActor))
  (`/Game/ThirdPersonBP/Blueprints/ThirdPersonCharacter.EquipWeapon` _asthird_person_character "NewEnumerator5")
  (`PrimitiveComponent.SetSimulatePhysics` (`self.Cube`) true)
  (set `/Game/ThirdPersonBP/Blueprints/ThirdPersonCharacter.isPushing` true _asthird_person_character))

(event `self.X Axis Collision1.OnComponentEndOverlap`
  (params (OverlappedComponent :type "PrimitiveComponent Object Reference") (OtherActor :type "Actor Object Reference") (OtherComp :type "PrimitiveComponent Object Reference") (OtherBodyIndex :type Integer))
  (bind _asthird_person_character (cast `/Game/ThirdPersonBP/Blueprints/ThirdPersonCharacter` OtherActor))
  (`PrimitiveComponent.SetSimulatePhysics` (`self.Cube`) false)
  (set `/Game/ThirdPersonBP/Blueprints/ThirdPersonCharacter.isPushing` false _asthird_person_character))

(fn `InteractWith`
  (params (Interactor :type "/Game/ThirdPersonBP/Blueprints/ThirdPersonCharacter Object Reference"))
  (returns (Success :type Boolean))
  (`/Game/Blueprints/InventorySystem/InventoryComponent.AddFunction` (`/Game/ThirdPersonBP/Blueprints/ThirdPersonCharacter.InventoryComponent` Interactor) "MovableCube" 1)
  (return true))

(fn `LookAt`
  (params (Observer :type "/Game/ThirdPersonBP/Blueprints/ThirdPersonCharacter Object Reference"))
  (returns (Message :type Text) (Item :type Name))
  (return "Hareket ettirilebilir kutu" "None"))

(fn `UserConstructionScript`)