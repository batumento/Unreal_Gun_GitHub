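; One-shot-at-a-time interactable push button for parkour levels that opens the wall and front door sharing its ButtonValue.
; InteractObjects locks CanPress and runs the ButtonAnimation macro, which plays a sound and lerps the button in and back out with timelines before re-enabling it.
; The macro's output, fired from timeline updates, finds the matching Wall_BP, opens it, switches the camera to it, opens the matching door and turns the spotlight green.
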(event `self.ReceiveBeginPlay`
  (bind (_returnvalue_location _returnvalue_rotation _returnvalue_scale) (`KismetMathLibrary.BreakTransform` (`SceneComponent.GetRelativeTransform` (`self.button`))))
  (set `self.OutButton` (`KismetMathLibrary.MakeTransform` _returnvalue_location _returnvalue_rotation _returnvalue_scale))
  (set `self.InButton` (`KismetMathLibrary.MakeTransform` (- _returnvalue_location (0.0 5.0 0.0)) _returnvalue_rotation _returnvalue_scale))
  (`self.EnableInput` (`GameplayStatics.GetPlayerController` 0)))

(event `/Game/Blueprints/InteractInterface.InteractObjects`
  (params (Player :type "Character Object Reference"))
  ;[1 1 1] Button Interaction(Push Button)
  (if (`self.canPress`)
    (set `self.canPress` false)
    ;[1 1 1] Button Moving Animation
    (`GameplayStatics.PlaySoundAtLocation` "/Game/ParkourActors/Buttons/SFX/buttonsfx.buttonsfx" (`self.K2_GetActorLocation`) (struct) 1.0 1.0 0.0 null null null)
    (bind (_direction _buttonin) (`Timeline|Button In` :!via `PlayFromStart`)
      (:`Update`
        (bind _returnvalue_location (`KismetMathLibrary.BreakTransform` (`KismetMathLibrary.TLerp` (`self.OutButton`) (`self.InButton`) _buttonin)))
        (`SceneComponent.K2_SetRelativeLocation` (`self.button`) _returnvalue_location false false)
        ;[1 1 1] butona bastığımda istediğim sifikifilişler olucak
        (bind _outactors (`GameplayStatics.GetAllActorsOfClass` "/Game/wall_BP.wall_BP_C" :!label _label))
        (for _array_element _outactors
          (if (== (`/Game/wall_BP.wallValue` _array_element) (`self.buttonValue`))
            (`|ExecutionSequence`
              (:`then_0`
                (`/Game/wall_BP.OpenWall` _array_element Player)
                (`PlayerController.SetViewTargetWithBlend` (`GameplayStatics.GetPlayerController` 0) _array_element 0.0 "VTBlend_Linear" 0.0 false)
                (bind _outactors_2 (`GameplayStatics.GetAllActorsOfClass` "/Game/ParkourActors/Door/FrontDoor_a_Blueprint.FrontDoor_a_Blueprint_C"))
                (for _array_element_2 _outactors_2
                  (if (== (`/Game/ParkourActors/Door/FrontDoor_a_Blueprint.doorValue` _array_element_2) (`self.buttonValue`))
                    (`/Game/ParkourActors/Door/FrontDoor_a_Blueprint.Open Door` _array_element_2)
                    (break)))
                (`LightComponent.SetLightColor` (`self.SpotLight`) (struct :`R` 0.088293 :`G` 1.0 :`A` 1.0) true))
              (:`then_1`
                (break))))))
      (:`Finished`
        (bind (_direction_2 _buttonin_2) (`Timeline|ButtonOut` :!via `ReverseFromEnd`)
          (:`Update`
            (bind _returnvalue_location_2 (`KismetMathLibrary.BreakTransform` (`KismetMathLibrary.TLerp` (`self.OutButton`) (`self.InButton`) _buttonin_2)))
            (`SceneComponent.K2_SetRelativeLocation` (`self.button`) _returnvalue_location_2 false false)
            (goto _label))
          (:`Finished`
            (set `self.canPress` true)))))))

(fn `UserConstructionScript`)